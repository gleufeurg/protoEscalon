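; Parent weapon pickup that equips itself on the first player and enters their inventory automatically shortly after BeginPlay, with no overlap or interaction check.
; PickupItem adds the BPCWeapon component to the player character, sets BP_Player's WeaponMesh from the DT_Item row named in Data, and returns that row name.
; BeginPlay then passes the row name and the pickup itself to the player's Inventory.
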(event EventBeginPlay
  (Utilities|FlowControl|Delay 0.2)
  (bind _row_name (CallFunction|PickupItem))
  (bind _asbp_player (Utilities|Casting|CastToBP_Player (Game|GetPlayerCharacter 0)))
  (Default|AddItemtoInventory (Variables|/Game/Player/Blueprints/BP_Player.BP_Player_C|GetInventory _asbp_player) _row_name self))

(fn ConstructionScript
  (|CallParentFunction))

(fn PickupItem
  (bind _returnvalue (Game|GetPlayerCharacter 0))
  (bind _data (Variables|Default|GetData))
  (Game|AddComponentbyClass _returnvalue (Variables|Default|GetBPC_Weapon))
  (bind _asbp_player (Utilities|Casting|CastToBP_Player _returnvalue))
  (bind _returnvalue_2 (Utilities|GetDataTableRow "/Game/Inventory/DT_Item.DT_Item" (.rowname _data))
    (:then
      (Components|StaticMesh|SetStaticMesh (Variables|/Game/Player/Blueprints/BP_Player.BP_Player_C|GetWeaponMesh _asbp_player) (.Mesh (Utilities|Struct|BreakF_Item _returnvalue_2)))
      (return (.rowname _data)))))