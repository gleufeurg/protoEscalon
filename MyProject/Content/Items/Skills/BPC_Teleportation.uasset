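; BPC_Teleportation is a skill component that blinks the player forward by a dash distance when used.
; On UseSkill it runs the parent logic, gets BP_Player, and line traces on the Visibility channel from the player's location along the forward vector.
; If the trace hits nothing, it teleports the player to the endpoint without sweeping; a blocked trace cancels the move rather than shortening it.
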(event EventBeginPlay
  (|CallParentFunction))

(event EventUseSkill
  (|CallParentFunction)
  (bind _asbp_player (Utilities|Casting|CastToBP_Player (Game|GetPlayerCharacter 0)))
  (bind _returnvalue (Collision|LineTraceByChannel (Transformation|GetActorLocation _asbp_player) (+ (Transformation|GetActorLocation _asbp_player) (* (Transformation|GetActorForwardVector _asbp_player) (Variables|Default|GetDash%20Dist))) "TraceTypeQuery1" false 0 "None"))
  (if (not _returnvalue)
    (Transformation|SetActorLocation _asbp_player (+ (Transformation|GetActorLocation _asbp_player) (* (Transformation|GetActorForwardVector _asbp_player) (Variables|Default|GetDash%20Dist))) false true)))