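; BPC_HeavySlash is a player skill component for a heavy slash attack.
; On use, it disables the player's weapon damage, spawns a BP_SlashHitbox carrying the skill's damage and gauge gain, and flashes a brief distortion effect ahead of it.
; Ending the skill restores weapon damage and destroys the hitbox.
; An older weapon-overlap damage handler remains, but its binding never runs.
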(event Custom|Weapon%20Overlap
  (params (OverlappedComponent :type Primitive%20Component%20Object%20Reference) (OtherActor :type Actor%20Object%20Reference) (OtherComp :type Primitive%20Component%20Object%20Reference) (OtherBodyIndex :type Integer) (bFromSweep :type Boolean) (SweepResult :type Hit%20Result%20Structure%20%28by%20ref%29))
  ;[1 1 1] Previous HeavySlash
  (bind _asbp_enemy_base (Utilities|Casting|CastToBP_Enemy_Base OtherActor))
  (Class|IDamageable|TakeDamage(Message) _asbp_enemy_base (Variables|Default|GetDamage) (Variables|Default|GetGaugeGain) 0.0 "0, 0, 0" 0.0)
  (Default|CallSlashDamage _asbp_enemy_base))

(event EventBeginPlay
  (|CallParentFunction))

(event EventUseSkill
  (|CallParentFunction)
  (bind _asbp_player (Utilities|Casting|CastToBP_Player (Components|GetOwner)))
  (Variables|/Game/Player/Blueprints/BP_Player.BP_Player_C|SetWeaponInflictDamage _asbp_player false)
  (bind _returnvalue (Game|SpawnActorfromClass "/Game/Items/Skills/HeavySlash/BP_SlashHitbox.BP_SlashHitbox_C" (Math|Transform|MakeTransform (.location (Transformation|GetActorTransform _asbp_player)) (.rotation (Transformation|GetActorTransform _asbp_player)) "1.000000,1.000000,1.000000") "AlwaysSpawn" "MultiplyWithRoot" 0 0))
  (bind _output_get (Variables|Default|SetHitbox _returnvalue))
  (Variables|/Game/Items/Skills/HeavySlash/BP_SlashHitbox.BP_SlashHitbox_C|SetDamage _output_get (Variables|Default|GetDamage))
  (Variables|/Game/Items/Skills/HeavySlash/BP_SlashHitbox.BP_SlashHitbox_C|SetGauge%20Gain _output_get (Variables|Default|GetGaugeGain))
  ;[1 1 1] Distorsion FX
  (bind _returnvalue_2 (Game|SpawnActorfromClass "/Game/FX/Effects/BP_Distorsion.BP_Distorsion_C" (Math|Transform|MakeTransform (+ (.location (Transformation|GetActorTransform _output_get)) (* (Transformation|GetActorForwardVector _output_get) 2.5e+02)) "0, 0, 0" "7.000000,7.000000,7.000000") "Undefined" "MultiplyWithRoot" 0 0))
  (Variables|Default|SetDistorsionFX _returnvalue_2)
  (Utilities|FlowControl|Delay 0.2)
  (Actor|DestroyActor (Variables|Default|GetDistorsionFX)))

(event EventEndSkill
  (|CallParentFunction)
  (bind _asbp_player (Utilities|Casting|CastToBP_Player (Components|GetOwner)))
  (Variables|/Game/Player/Blueprints/BP_Player.BP_Player_C|SetWeaponInflictDamage _asbp_player true)
  (Actor|DestroyActor (Variables|Default|GetHitbox)))