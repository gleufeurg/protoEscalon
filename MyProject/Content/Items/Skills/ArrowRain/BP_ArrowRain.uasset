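; BP_ArrowRain is an area skill actor that deals periodic damage to enemies inside its hit box, then destroys itself after a set number of ticks.
; On spawn it plays a camera shake and activation sound, and overlap events maintain the list of enemies in range.
; A Running/Ended timer state driven by Tick counts down between pulses, each replaying the sound and sending damage and gauge gain to those enemies.
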(event OnComponentBeginOverlap(HitBox)
  (params (OverlappedComponent :type Primitive%20Component%20Object%20Reference) (OtherActor :type Actor%20Object%20Reference) (OtherComp :type Primitive%20Component%20Object%20Reference) (OtherBodyIndex :type Integer) (bFromSweep :type Boolean) (SweepResult :type Hit%20Result%20Structure%20%28by%20ref%29))
  (bind _asbp_enemy_base (Utilities|Casting|CastToBP_Enemy_Base OtherActor))
  (Utilities|Array|Add (Variables|Default|GetEnemiesInRange) _asbp_enemy_base))

(event OnComponentEndOverlap(HitBox)
  (params (OverlappedComponent :type Primitive%20Component%20Object%20Reference) (OtherActor :type Actor%20Object%20Reference) (OtherComp :type Primitive%20Component%20Object%20Reference) (OtherBodyIndex :type Integer))
  (bind _asbp_enemy_base (Utilities|Casting|CastToBP_Enemy_Base OtherActor))
  (Utilities|Array|RemoveItem (Variables|Default|GetEnemiesInRange) _asbp_enemy_base))

(event Custom|Effect
  (Audio|PlaySoundatLocation "/Game/FX/Sounds/SoundWaves/Player/Skills/ArrowRain/Skill_Arrow_Activation.Skill_Arrow_Activation" (Transformation|GetActorLocation) "0, 0, 0" 1.0 1.0 0.0 0 0 0 0)
  (for _array_element (Variables|Default|GetEnemiesInRange)
    (Class|IDamageable|TakeDamage(Message) _array_element (Variables|Default|GetDamage) (Variables|Default|GetGaugeGain))))

(event EventTick
  (params (DeltaSeconds :type Float%20%28single-precision%29))
  (switch Utilities|FlowControl|Switch|SwitchonETimerState (Variables|Default|GetTimer)
    (:NewEnumerator0
      (bind _output_get (Variables|Default|SetCooldown%20Time (- (Variables|Default|GetCooldown%20Time) DeltaSeconds)))
      (if (<= _output_get 0.0)
        (Variables|Default|SetTimer "NewEnumerator1")))
    (:NewEnumerator1
      (CallFunction|Effect)
      (bind _output_get_2 (Variables|Default|SetTickCount (+ (Variables|Default|GetTickCount) 1)))
      (if (>= _output_get_2 (Variables|Default|GetMaxTick))
        (Actor|DestroyActor)
        (else
          (Variables|Default|SetCooldown%20Time (Variables|Default|GetMaxTime))
          (Variables|Default|SetTimer "NewEnumerator0"))))))

(event EventBeginPlay
  (Variables|Default|SetCooldown%20Time (Variables|Default|GetMaxTime))
  (Camera|PlayWorldCameraShake "/Game/FX/Effects/Camera/CS_TakeDamage.CS_TakeDamage_C" (Transformation|GetActorLocation) 0.0 3e+03)
  (Audio|PlaySoundatLocation "/Game/FX/Sounds/SoundWaves/Player/Skills/ArrowRain/Skill_Arrow_Activation.Skill_Arrow_Activation" (Transformation|GetActorLocation) "0, 0, 0" 1.0 1.0 0.0 0 0 0 0))

(fn ConstructionScript)