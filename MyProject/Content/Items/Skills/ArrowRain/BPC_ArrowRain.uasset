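; Arrow Rain skill component that extends a parent skill and spawns an arrow rain actor at the owning player's target location.
; On use, it casts the owner to BP_Player, spawns the actor, then passes it the tick interval, tick count, damage and gauge gain.
; A comment plans mouse-based targeting within a radius around the player, and an unconnected Niagara spawn node never runs.
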(event EventBeginPlay
  (|CallParentFunction))

(event EventUseSkill
  (|CallParentFunction)
  ;[0 0 0 0.85] A changer avec le target system via la souris
  ; Le prochain systeme fera en sorte de cast le skill là où la souris est (dans un rayion défini autour du joueur)
  (bind _asbp_player (Utilities|Casting|CastToBP_Player (Components|GetOwner)))
  (bind _returnvalue (Game|SpawnActorfromClass (Variables|Default|GetArrowRain) (Math|Transform|MakeTransform (Variables|/Game/Player/Blueprints/BP_Player.BP_Player_C|GetTarget%20Loc _asbp_player) "0, 0, 0" "1.000000,1.000000,1.000000") "AlwaysSpawn" "MultiplyWithRoot" 0 0))
  (bind _output_get (Variables|Default|SetSpawnedArrow _returnvalue))
  (bind _asbp_arrow_rain (Utilities|Casting|CastToBP_ArrowRain _output_get))
  ;[1 1 1] Need to set this up
  (bind _output_get_2 (Variables|/Game/Items/Skills/ArrowRain/BP_ArrowRain.BP_ArrowRain_C|SetCooldown%20Time _asbp_arrow_rain (Variables|Ticks|GetTickDuration)))
  (Variables|/Game/Items/Skills/ArrowRain/BP_ArrowRain.BP_ArrowRain_C|SetMaxTime _asbp_arrow_rain _output_get_2)
  (Variables|/Game/Items/Skills/ArrowRain/BP_ArrowRain.BP_ArrowRain_C|SetMaxTick _asbp_arrow_rain (Variables|Ticks|GetNumberOfActivations))
  (Variables|/Game/Items/Skills/ArrowRain/BP_ArrowRain.BP_ArrowRain_C|SetDamage _asbp_arrow_rain (Variables|Default|GetDamage))
  (Variables|/Game/Items/Skills/ArrowRain/BP_ArrowRain.BP_ArrowRain_C|SetGaugeGain _asbp_arrow_rain (Variables|Default|GetGaugeGain)))