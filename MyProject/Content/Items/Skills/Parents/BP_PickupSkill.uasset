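; BP_PickupSkill is a parent Blueprint for skill pickups that grant the player a skill.
; Shortly after BeginPlay, it calls PickupItem, which adds a component of the BPCSkill class to the player character and appends it to the player's Skills list.
; It then passes the returned data row name and itself to the player's Inventory to register the item.
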(event EventBeginPlay
  (Utilities|FlowControl|Delay 0.2)
  (bind _row_name (CallFunction|PickupItem))
  (bind _asbp_player (Utilities|Casting|CastToBP_Player (Game|GetPlayerCharacter 0)))
  (Default|AddItemtoInventory (Variables|/Game/Player/Blueprints/BP_Player.BP_Player_C|GetInventory _asbp_player) _row_name self))

(fn ConstructionScript
  (|CallParentFunction))

(fn PickupItem
  (bind _returnvalue (Game|GetPlayerCharacter 0))
  (bind _returnvalue_2 (Game|AddComponentbyClass _returnvalue (Variables|Default|GetBPC_Skill)))
  (bind _asbp_player (Utilities|Casting|CastToBP_Player _returnvalue))
  (Utilities|Array|Add (Variables|/Game/Player/Blueprints/BP_Player.BP_Player_C|GetSkills _asbp_player) _returnvalue_2)
  (return (.rowname (Variables|Default|GetData))))