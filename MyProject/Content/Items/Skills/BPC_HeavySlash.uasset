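; Heavy Slash skill component for the player that turns weapon hits into skill damage while the slash is active.
; UseSkill switches off the player's normal weapon damage and binds WeaponOverlap to the weapon mesh's begin-overlap event.
; Each enemy overlap sends the skill's damage and gauge gain to that enemy and calls the SlashDamage dispatcher.
; EndHeavySlash unbinds the overlap and restores normal weapon damage.
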(event Custom|End%20Heavy%20Slash
  (bind _asbp_player (Utilities|Casting|CastToBP_Player (Components|GetOwner)))
  (Collision|UnbindEventfromOnComponentBeginOverlap (Variables|/Game/Player/Blueprints/BP_Player.BP_Player_C|GetWeaponMesh _asbp_player) (delegate Custom|Weapon%20Overlap))
  (Variables|/Game/Player/Blueprints/BP_Player.BP_Player_C|SetWeaponInflictDamage _asbp_player true))

(event Custom|Weapon%20Overlap
  (params (OverlappedComponent :type Primitive%20Component%20Object%20Reference) (OtherActor :type Actor%20Object%20Reference) (OtherComp :type Primitive%20Component%20Object%20Reference) (OtherBodyIndex :type Integer) (bFromSweep :type Boolean) (SweepResult :type Hit%20Result%20Structure%20%28by%20ref%29))
  (bind _asbp_enemy_base (Utilities|Casting|CastToBP_Enemy_Base OtherActor))
  (Class|IDamageable|TakeDamage(Message) _asbp_enemy_base (Variables|Default|GetDamage) (Variables|Default|GetGaugeGain))
  (Default|CallSlashDamage _asbp_enemy_base))

(event EventBeginPlay
  (|CallParentFunction))

(event EventUseSkill
  (|CallParentFunction)
  (bind _asbp_player (Utilities|Casting|CastToBP_Player (Components|GetOwner)))
  (Variables|/Game/Player/Blueprints/BP_Player.BP_Player_C|SetWeaponInflictDamage _asbp_player false)
  (Collision|AssignOnComponentBeginOverlap (Variables|/Game/Player/Blueprints/BP_Player.BP_Player_C|GetWeaponMesh _asbp_player) (delegate Custom|Weapon%20Overlap)))