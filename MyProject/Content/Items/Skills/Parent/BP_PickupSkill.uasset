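; Parent skill pickup that grants the player a skill component and an inventory entry shortly after it begins play.
; PickupItem adds the BPCSkill component to the player character, then looks up its row in DT_Item.
; For Skill-type rows, the component fills the Skills slot at ItemOrder, or is appended if that slot is occupied.
; The returned row name is then passed to the player's Inventory along with the pickup itself.
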(event EventBeginPlay
  (Utilities|FlowControl|Delay 0.2)
  (bind _row_name (CallFunction|PickupItem))
  (bind _asbp_player (Utilities|Casting|CastToBP_Player (Game|GetPlayerCharacter 0)))
  (Default|AddItemtoInventory (Variables|/Game/Player/Blueprints/BP_Player.BP_Player_C|GetInventory _asbp_player) _row_name self))

(fn ConstructionScript
  (|CallParentFunction))

(fn PickupItem
  (bind _returnvalue (Game|GetPlayerCharacter 0))
  (bind _data (Variables|Default|GetData))
  (bind _returnvalue_2 (Game|AddComponentbyClass _returnvalue (Variables|Default|GetBPC_Skill)))
  (bind _asbp_player (Utilities|Casting|CastToBP_Player _returnvalue))
  (bind _returnvalue_3 (Utilities|GetDataTableRow "/Game/Inventory/DT_Item.DT_Item" (.rowname _data))
    (:then
      (switch Utilities|FlowControl|Switch|SwitchonE_ItemType (.Type (Utilities|Struct|BreakF_Item _returnvalue_3))
        (:NewEnumerator0
          (Utilities|IsValid (Utilities|Array|Get(acopy) (Variables|/Game/Player/Blueprints/BP_Player.BP_Player_C|GetSkills _asbp_player) (.ItemOrder (Utilities|Struct|BreakF_Item _returnvalue_3)))
            (:Is%20Valid
              (Utilities|Array|Add (Variables|/Game/Player/Blueprints/BP_Player.BP_Player_C|GetSkills _asbp_player) _returnvalue_2))
            (:Is%20Not%20Valid
              (Utilities|Array|SetArrayElem (Variables|/Game/Player/Blueprints/BP_Player.BP_Player_C|GetSkills _asbp_player) (.ItemOrder (Utilities|Struct|BreakF_Item _returnvalue_3)) _returnvalue_2 true)))
          (return (.rowname _data)))))))