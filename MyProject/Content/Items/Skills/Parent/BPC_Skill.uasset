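; Parent component for player skills, providing shared stat setup and use, end and cancel events.
; On BeginPlay it loads cost, damage and gauge gain from its DT_Item row, then lets each of the player's ring components modify its passives.
; UseSkill spends the player's gauge points by cost, then triggers each ring's active modifiers for the skill and player.
; EndSkill and CancelSkill are empty here.
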(event Custom|Use%20Skill
  (bind _asbp_player (Utilities|Casting|CastToBP_Player (Components|GetOwner)))
  (Default|LoseGaugePoints _asbp_player (Variables|Default|GetCost))
  (for _array_element (Variables|/Game/Player/Blueprints/BP_Player.BP_Player_C|GetBPC_Rings _asbp_player)
    (Default|ModifyActive _array_element self)
    (Default|ModifyPlayerActive _array_element)))

(event Custom|Cancel%20Skill)

(event Custom|End%20Skill)

(event EventBeginPlay
  (bind _returnvalue (Utilities|GetDataTableRow "/Game/Inventory/DT_Item.DT_Item" (.rowname (Variables|Default|GetData)))
    (:then
      (Variables|Default|SetCost (.Cost (Utilities|Struct|BreakF_Item _returnvalue)))
      (Variables|Default|SetDamage (.Damage (Utilities|Struct|BreakF_Item _returnvalue)))
      (Variables|Default|SetGaugeGain (.GaugeGain (Utilities|Struct|BreakF_Item _returnvalue)))
      (bind _asbp_player (Utilities|Casting|CastToBP_Player (Components|GetOwner)))
      (for _array_element (Variables|/Game/Player/Blueprints/BP_Player.BP_Player_C|GetBPC_Rings _asbp_player)
        (Default|ModifyPassives _array_element self)))))