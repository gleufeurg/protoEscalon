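; Ring item component that leaves a trail of damaging fire behind the moving player.
; On BeginPlay it starts a looping timer at FireRate, which spawns a BP_FireStep actor at foot level behind the player whenever velocity is non-zero.
; Each spawned fire receives its lifespan, damage, gauge gain and effect duration from the component.
; ModifyPassives zeroes the Dash component's distance when one is valid.
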(event Custom|Fire
  (bind _player (Variables|Default|GetPlayer))
  (if (> (Math|Vector|VectorLength (Variables|/Script/Engine.MovementComponent|GetVelocity (Variables|/Script/Engine.Character|GetCharacterMovement _player))) 0.0)
    (bind _returnvalue (Game|SpawnActorfromClass "/Game/Items/Rings/Dash/BP_FireStep.BP_FireStep_C" (Math|Transform|MakeTransform (- (- (Transformation|GetActorLocation _player) "0.000000,0.000000,50.000000") (* (Transformation|GetActorForwardVector _player) 1e+02)) "0, 0, 0" "1.000000,1.000000,1.000000") "Undefined" "MultiplyWithRoot" 0 0))
    (Actor|SetLifeSpan _returnvalue (Variables|Default|GetDuration))
    (Variables|/Game/Items/Rings/Dash/BP_FireStep.BP_FireStep_C|SetDamage _returnvalue (Variables|Default|GetDamage))
    (Variables|/Game/Items/Rings/Dash/BP_FireStep.BP_FireStep_C|SetGauge%20Gain _returnvalue (Variables|Default|GetGauge%20Gain))
    (Effects|Components|ParticleSystem|SetFloatParameter (Variables|/Game/Items/Rings/Dash/BP_FireStep.BP_FireStep_C|GetFire _returnvalue) "Duration" (Variables|Default|GetDuration))))

(event EventBeginPlay
  (|CallParentFunction)
  (Utilities|Time|SetTimerbyEvent (delegate Custom|Fire) (Variables|Default|GetFireRate) true)
  (bind _returnvalue (Utilities|GetDataTableRow "/Game/Inventory/DT_Item.DT_Item" (.rowname (Variables|Default|GetData)))))

(event EventModifyPassives
  (params (BPC_Skill :type BPC%20Skill%20Object%20Reference))
  (bind _dash (Variables|Default|GetDash))
  (Utilities|IsValid _dash
    (:Is%20Valid
      (Variables|/Game/Items/Skills/Dash/BPC_Dash.BPC_Dash_C|SetDash%20Dist _dash 0.0))))