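; BPC_Hungry is a Slash ring modifier that makes the Heavy Slash skill costlier and far more damaging.
; On ModifyPassives it casts the given skill to BPC_HeavySlash, adds a small flat amount to Cost and applies a large multiplier to Damage.
; Other skills fail the cast and are left untouched.
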(event EventBeginPlay
  (|CallParentFunction) ; This node is disabled and will not be called.\nDrag off pins to build functionality.
)

(event EventTick
  (params (DeltaSeconds :type Float%20%28single-precision%29))
  (|CallParentFunction DeltaSeconds) ; This node is disabled and will not be called.\nDrag off pins to build functionality.
)

(event EventModifyPassives
  (params (BPC_Skill :type BPC%20Skill%20Object%20Reference))
  (bind _asbpc_heavy_slash (Utilities|Casting|CastToBPC_HeavySlash BPC_Skill))
  (Variables|/Game/Items/Skills/Parent/BPC_Skill.BPC_Skill_C|SetCost _asbpc_heavy_slash (+ (Variables|/Game/Items/Skills/Parent/BPC_Skill.BPC_Skill_C|GetCost _asbpc_heavy_slash) 0.02))
  (Variables|/Game/Items/Skills/Parent/BPC_Skill.BPC_Skill_C|SetDamage _asbpc_heavy_slash (* (Variables|/Game/Items/Skills/Parent/BPC_Skill.BPC_Skill_C|GetDamage _asbpc_heavy_slash) 5e+01)))