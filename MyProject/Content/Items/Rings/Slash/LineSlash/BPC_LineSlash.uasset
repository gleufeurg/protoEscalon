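; Ring item component for the Line Slash ring, whose active effect spawns a slash actor in front of the player.
; ModifyActive spawns BP_LineSlash at an offset along the player's forward vector, matching the player's rotation and ignoring collisions, then passes it the component's Damage.
; BeginPlay defers to the parent, and ModifyPassives is empty, so the ring adds no passive effect here.
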(event EventBeginPlay
  (|CallParentFunction))

(event EventModifyPassives
  (params (BPC_Skill :type BPC%20Skill%20Object%20Reference)))

(event EventModifyActive
  (params (BPC_Skill :type BPC%20Skill%20Object%20Reference))
  (bind _player (Variables|Default|GetPlayer))
  (bind _returnvalue (Transformation|GetActorTransform _player))
  (bind _returnvalue_2 (Game|SpawnActorfromClass "/Game/Items/Rings/Slash/LineSlash/BP_LineSlash.BP_LineSlash_C" (Math|Transform|MakeTransform (+ (.location _returnvalue) (* (Transformation|GetActorForwardVector _player) (Variables|Default|GetSpawnOffset))) (.rotation _returnvalue) "1.000000,1.000000,1.000000") "AlwaysSpawn" "MultiplyWithRoot" 0 0))
  (Variables|/Game/Items/Rings/Slash/LineSlash/BP_LineSlash.BP_LineSlash_C|SetDamage _returnvalue_2 (Variables|Default|GetDamage)))