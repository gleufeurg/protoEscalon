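; BPC_Sleep is a ring component, apparently meant to give the player's Heavy Slash a chance to put hit actors to sleep.
; On BeginPlay it searches the owning player's Skills for BPC_HeavySlash and binds its Sleep event to that skill's slash damage.
; Sleep rolls a one-in-three chance on each call, but the success branch is empty, so no effect is applied yet.
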(event Custom|Sleep
  (params (ActorHitted :type BP%20Enemy%20Base%20Object%20Reference))
  (if (<= (Math|Random|RandomFloat) (/ (Math|Float|MakeLiteralFloat 1.0) (Math|Float|MakeLiteralFloat 3.0)))
    _))

(event EventBeginPlay
  (|CallParentFunction)
  (bind _asbp_player (Utilities|Casting|CastToBP_Player (Components|GetOwner)))
  (bind _output_get (Variables|Default|SetAs%20BP%20Player _asbp_player))
  (for _array_element (Variables|/Game/Player/Blueprints/BP_Player.BP_Player_C|GetSkills _output_get)
    (bind _asbpc_heavy_slash (Utilities|Casting|CastToBPC_HeavySlash _array_element))
    (EventDispatchers|BindEventtoSlashDamage _asbpc_heavy_slash (delegate Custom|Sleep))))

(event EventTick
  (params (DeltaSeconds :type Float%20%28single-precision%29)))