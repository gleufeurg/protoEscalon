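; Base component for rings that modify the player's skills and stats, with empty passive, active and reset hooks, presumably for child rings to override.
; On BeginPlay it caches the player's Dash, ArrowRain and HeavySlash skills, registers itself in the player's Rings, then runs the passive hooks on each skill and the player.
; It also spawns a ring actor on a random socket of the owner's mesh with a random-hue point light aura.
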(event Custom|Modify%20Passives
  (params (BPC_Skill :type BPC%20Skill%20Object%20Reference))
  ;[0 0 0 0.85] Modify Skills stats and everything before Skill Activation
)

(event Custom|Modify%20Active
  (params (BPC_Skill :type BPC%20Skill%20Object%20Reference))
  ;[0 0 0 0.85] Special effects during Skill Activation
  ; Used for hard skills modifiers
)

(event Custom|Modify%20Player%20Active)

(event Custom|Reset%20Modifiers)

(event Custom|Modify%20Player%20Passives)

(event EventBeginPlay
  (bind _asbp_player (Utilities|Casting|CastToBP_Player (Game|GetPlayerCharacter 0)))
  (Variables|Default|SetPlayer _asbp_player)
  (CallFunction|SetSkillsRefs)
  (CallFunction|ModifyPassivestoAll)
  (CallFunction|ModifyPlayerPassives)
  (bind _asbp_player_2 (Utilities|Casting|CastToBP_Player (Components|GetOwner)))
  ;[0 0 0] Atttach to fingers
  (bind _returnvalue (Game|SpawnActorfromClass "/Game/Items/Rings/Parents/BP_RingAttached.BP_RingAttached_C" (Math|Transform|MakeTransform "0, 0, 0" "0, 0, 0" "1.000000,1.000000,1.000000") "Undefined" "MultiplyWithRoot" 0 0))
  (Transformation|AttachComponentToComponent _returnvalue (Variables|/Script/Engine.Character|GetMesh _asbp_player_2) (.OutItem (Utilities|Array|Random (Variables|Default|GetSockets))) "SnapToTarget" "SnapToTarget" "KeepRelative" true)
  ;[1 1 1] Set Aura
  (Class|KismetMathLibrary|LinearColorSetRandomHue (Variables|Default|GetColor))
  (Rendering|Components|Light|SetLightColor (Variables|/Game/Items/Rings/Parents/BP_RingAttached.BP_RingAttached_C|GetPointLight _returnvalue) (Variables|Default|GetColor) true))

(fn ModifyPassivestoAll
  (bind _player (Variables|Default|GetPlayer))
  (Utilities|Array|Add (Variables|/Game/Player/Blueprints/BP_Player.BP_Player_C|GetRings _player) self)
  ;[0 0 0 0.85] Modify skills passives (Stats...)
  (for _array_element (Variables|/Game/Player/Blueprints/BP_Player.BP_Player_C|GetSkills _player)
    (CallFunction|ModifyPassives _array_element)))

(fn SetSkillsRefs
  (for _array_element (Variables|/Game/Player/Blueprints/BP_Player.BP_Player_C|GetSkills (Variables|Default|GetPlayer))
    (bind _asbpc_dash (Utilities|Casting|CastToBPC_Dash _array_element)
      (:then
        (Variables|Default|SetDash _asbpc_dash))
      (:CastFailed
        (bind _asbpc_arrow_rain (Utilities|Casting|CastToBPC_ArrowRain _array_element)
          (:then
            (Variables|Default|SetArrowRain _asbpc_arrow_rain))
          (:CastFailed
            (bind _asbpc_heavy_slash (Utilities|Casting|CastToBPC_HeavySlash _array_element))
            (Variables|Default|SetSlash _asbpc_heavy_slash)))))))