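; BP_Meteor is a meteor strike actor that falls onto its spawn location and deals heavy damage to enemies in its radius.
; On BeginPlay it sizes the hitbox, teleports up by an offset, and a timeline sweeps it back to the target.
; Hitbox overlaps maintain the list of enemies in range.
; When the fall finishes, it spawns the impact Niagara effect, damages that list with a freeze-frame, and destroys itself.
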(event OnComponentBeginOverlap(Hitbox)
  (params (OverlappedComponent :type Primitive%20Component%20Object%20Reference) (OtherActor :type Actor%20Object%20Reference) (OtherComp :type Primitive%20Component%20Object%20Reference) (OtherBodyIndex :type Integer) (bFromSweep :type Boolean) (SweepResult :type Hit%20Result%20Structure%20%28by%20ref%29))
  (bind _asbp_enemy_base (Utilities|Casting|CastToBP_Enemy_Base OtherActor))
  (Utilities|Array|Add (Variables|Default|GetEnemiesHit) _asbp_enemy_base))

(event OnComponentEndOverlap(Hitbox)
  (params (OverlappedComponent :type Primitive%20Component%20Object%20Reference) (OtherActor :type Actor%20Object%20Reference) (OtherComp :type Primitive%20Component%20Object%20Reference) (OtherBodyIndex :type Integer))
  (bind _asbp_enemy_base (Utilities|Casting|CastToBP_Enemy_Base OtherActor))
  (Utilities|Array|RemoveItem (Variables|Default|GetEnemiesHit) _asbp_enemy_base))

(event Custom|Impact
  (Niagara|SpawnSystematLocation "/Game/Items/Rings/ArrowRain/Meteor/NS_Meteor_Impact.NS_Meteor_Impact" (Variables|Default|GetEndLoc))
  (for _array_element (Variables|Default|GetEnemiesHit)
    (Class|IDamageable|TakeDamage(Message) _array_element 2.5e+04 0.0 0.0 "0, 0, 0" 0.5))
  (Actor|DestroyActor))

(event EventBeginPlay
  (Components|Sphere|SetSphereRadius (Variables|Default|GetHitbox) (Variables|Default|GetRadius) true)
  (bind _output_get (Variables|Default|SetEndLoc (Transformation|GetActorLocation)))
  (bind _output_get_2 (Variables|Default|SetStartLoc (+ _output_get (Variables|Default|GetOffsetLoc))))
  (Transformation|SetActorLocation _output_get_2 false true)
  (bind _fall (Timeline|MeteorFall PlayFromStart)
    (:Update
      (Transformation|SetActorLocationAndRotation (Math|Vector|Lerp(Vector) (Variables|Default|GetStartLoc) (Variables|Default|GetEndLoc) _fall) "0, 0, 0" true))
    (:Finished
      (CallFunction|Impact))))

(fn ConstructionScript)