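; BP_Vortex is a timed vortex from the ArrowRain ring item that pulls enemies toward its center.
; On BeginPlay, Radius sizes both the overlap sphere and the NSVortex effect, and Duration sets its lifespan.
; Sphere overlaps maintain a list of BP_Enemy_Base actors inside.
; Every Tick, each listed enemy receives an additive LaunchCharacter toward the center scaled by Strength, without delta-time scaling.
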(event OnComponentBeginOverlap(Sphere)
  (params (OverlappedComponent :type Primitive%20Component%20Object%20Reference) (OtherActor :type Actor%20Object%20Reference) (OtherComp :type Primitive%20Component%20Object%20Reference) (OtherBodyIndex :type Integer) (bFromSweep :type Boolean) (SweepResult :type Hit%20Result%20Structure%20%28by%20ref%29))
  (bind _asbp_enemy_base (Utilities|Casting|CastToBP_Enemy_Base OtherActor))
  (Utilities|Array|AddUnique (Variables|Default|GetActorInVortex) _asbp_enemy_base))

(event OnComponentEndOverlap(Sphere)
  (params (OverlappedComponent :type Primitive%20Component%20Object%20Reference) (OtherActor :type Actor%20Object%20Reference) (OtherComp :type Primitive%20Component%20Object%20Reference) (OtherBodyIndex :type Integer))
  (bind _asbp_enemy_base (Utilities|Casting|CastToBP_Enemy_Base OtherActor))
  (Utilities|Array|RemoveItem (Variables|Default|GetActorInVortex) _asbp_enemy_base))

(event EventBeginPlay
  (Components|Sphere|SetSphereRadius (Variables|Default|GetSphere) (Variables|Default|GetRadius) true)
  (Actor|SetLifeSpan (Variables|Default|GetDuration))
  (Niagara|SetNiagaraVariable(Float) (Variables|Default|GetNS_Vortex) "Size" (Variables|Default|GetRadius)))

(event EventTick
  (params (DeltaSeconds :type Float%20%28single-precision%29))
  (for _array_element (Variables|Default|GetActorInVortex)
    (Character|LaunchCharacter _array_element (* (Math|Vector|GetUnitDirection(Vector) (Transformation|GetActorLocation _array_element) (Transformation|GetWorldLocation (Variables|Default|GetSphere))) (Variables|Default|GetStrength)) false false)))

(fn ConstructionScript)