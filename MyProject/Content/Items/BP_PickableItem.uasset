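; BP_PickableItem is a world item actor that can be picked up and identifies itself by a row in the DT_Item data table.
; Its construction script looks up that row and applies its artwork as the Tex parameter of a transient dynamic material instance on the static mesh.
; PickupItem only returns the row name, leaving any further pickup handling outside this Blueprint.
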(fn ConstructionScript
  (bind _returnvalue (Utilities|GetDataTableRow "/Game/Inventory/DT_Item.DT_Item" (.rowname (Variables|Default|GetData)))
    (:then
      (bind _returnvalue_2 (Rendering|Material|CreateDynamicMaterialInstance (Rendering|Material|GetMaterial (Variables|Default|GetStaticMesh) 0) "MI_PickableItem" "Transient" :!class /Script/Engine.KismetMaterialLibrary))
      (Rendering|Material|SetTextureParameterValue _returnvalue_2 "Tex" (.Artwork (Utilities|Struct|BreakF_Item _returnvalue)))
      (Rendering|Material|SetMaterial (Variables|Default|GetStaticMesh) 0 _returnvalue_2))))

(fn PickupItem
  (return (.rowname (Variables|Default|GetData))))