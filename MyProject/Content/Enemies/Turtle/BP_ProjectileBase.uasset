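; Base projectile Blueprint in the Turtle enemy folder, with a helper to keep it at a set height over the ground.
; SetAtRightGroundDistance line-traces vertically for a "Ground"-tagged actor and resets Z to GroundDist above that actor's origin when the gap exceeds GroundDist.
; The trace end scales with the projectile's own Z, and height is measured from the actor's origin rather than the impact point.
; Hit and BeginPlay are empty, and nothing here calls the helper.
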(event EventBeginPlay)

(event Collision|EventHit
  (params (MyComp :type Primitive%20Component%20Object%20Reference) (Other :type Actor%20Object%20Reference) (OtherComp :type Primitive%20Component%20Object%20Reference) (bSelfMoved :type Boolean) (HitLocation :type Vector :default "0, 0, 0") (HitNormal :type Vector :default "0, 0, 0") (NormalImpulse :type Vector :default "0, 0, 0") (Hit :type Hit%20Result%20Structure%20%28by%20ref%29)))

(fn ConstructionScript)

(fn SetatRightGroundDistance
  (bind _returnvalue (Transformation|GetActorLocation))
  (bind _returnvalue_2 (Transformation|GetActorLocation))
  (bind _outhit (Collision|LineTraceByChannel (Math|Vector|MakeVector (.x _returnvalue_2) (.y _returnvalue_2) (.z _returnvalue_2)) (Math|Vector|MakeVector (.x _returnvalue_2) (.y _returnvalue_2) (- (.z _returnvalue_2) (* (.z _returnvalue_2) 5e+02))) "TraceTypeQuery1" false 0 "None"))
  (Utilities|IsValid (.HitActor (Collision|BreakHitResult _outhit))
    (:Is%20Valid
      (if (Actor|ActorHasTag (.HitActor (Collision|BreakHitResult _outhit)) "Ground")
        (if (> (Math|Float|Absolute(Float) (- (.z (Transformation|GetActorLocation (.HitActor (Collision|BreakHitResult _outhit)))) (.z _returnvalue))) (Variables|Default|GetgroundDist))
          (Transformation|SetActorLocation (Math|Vector|MakeVector (.x _returnvalue) (.y _returnvalue) (+ (.z (Transformation|GetActorLocation (.HitActor (Collision|BreakHitResult _outhit)))) (Variables|Default|GetgroundDist))) false false))))))