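; BP_Turtle is an enemy Blueprint that makes a ranged attack by firing a projectile.
; Its Attack event calls the parent, then computes a spawn location and rotation from the capsule's rotation and the projectile offset.
; It always spawns a BP_ProjectileBase there, passing itself as the owning enemy along with its damage value.
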(event EventAttack
  (bind _capsulecomponent (Variables|Default|GetCapsuleComponent))
  (|CallParentFunction)
  (bind (_location _rotation) (CallFunction|Target _capsulecomponent (Variables|Default|GetProjectileOffset) (Transformation|GetWorldRotation _capsulecomponent)))
  (bind _returnvalue (Game|SpawnActorfromClass "/Game/Enemies/Turtle/BP_ProjectileBase.BP_ProjectileBase_C" (Math|Transform|MakeTransform _location _rotation "1.000000,1.000000,1.000000") "AlwaysSpawn" "OverrideRootScale" 0 0))
  (Variables|/Game/Enemies/Turtle/BP_ProjectileBase.BP_ProjectileBase_C|SetEnemy _returnvalue self)
  (Variables|/Game/Enemies/Turtle/BP_ProjectileBase.BP_ProjectileBase_C|SetDamage _returnvalue (Variables|Stats|Attack|GetDamage_0_0)))

(fn ConstructionScript
  (|CallParentFunction))