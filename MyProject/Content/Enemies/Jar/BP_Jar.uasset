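; BP_Jar is a breakable jar, filed under enemies, that shatters when it takes any damage.
; Its construction script gives it a random mesh from a Meshes array for visual variety.
; On damage it calls Die, which fires the OnDie dispatcher and destroys the actor, and it plays a shatter sound at its location.
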(event EventBeginPlay
  (|CallParentFunction))

(event EventTakeDamage
  (params (Damage :type Float%20%28double-precision%29) (GaugeGain :type Float%20%28double-precision%29) (KB%20Strength :type Float%20%28double-precision%29) (KB%20Direction :type Vector :default "0, 0, 0") (FreezeFrameDurationDuration :type Float%20%28double-precision%29) (RadialBlurDuration :type Float%20%28double-precision%29) (ChromaAberrationDuration :type Float%20%28double-precision%29) (FreezeFrame :type Boolean) (CameraShake :type Boolean) (RadialBlur :type Boolean) (ChromaAberration :type Boolean))
  (CallFunction|Die)
  (Audio|PlaySoundatLocation "/Game/FX/Sounds/Enemies/SC_JarShatter.SC_JarShatter" (Transformation|GetActorLocation) "0, 0, 0" 1.0 1.0 0.0 0 0 0 0))

(event EventDie
  (Default|CallOnDie self)
  (Actor|DestroyActor))

(fn ConstructionScript
  (|CallParentFunction)
  (Components|StaticMesh|SetStaticMesh (Variables|Default|GetJar) (.OutItem (Utilities|Array|Random (Variables|Default|GetMeshes)))))