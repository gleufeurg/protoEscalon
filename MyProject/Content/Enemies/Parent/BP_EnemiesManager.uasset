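; BP_EnemiesManager is an enemy manager Blueprint that holds per-team data for seven phonetically named teams, Alpha through Golf.
; Its only logic is GetTeam, which switches on a team value and returns the matching member variable.
; BeginPlay and the construction script are empty, so the file itself does no spawning, registration or updating of teams.
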(event EventBeginPlay)

(fn ConstructionScript)

(fn GetTeam
  (params (Team :type E_Team%20Enum :default "NewEnumerator0"))
  (switch Utilities|FlowControl|Switch|SwitchonE_Team Team
    (:NewEnumerator0
      (return (Variables|Teams|GetAlpha)))
    (:NewEnumerator1
      (return (Variables|Teams|GetBravo)))
    (:NewEnumerator2
      (return (Variables|Teams|GetCharlie)))
    (:NewEnumerator3
      (return (Variables|Teams|GetDelta)))
    (:NewEnumerator4
      (return (Variables|Teams|GetEcho)))
    (:NewEnumerator5
      (return (Variables|Teams|GetFoxTrot)))
    (:NewEnumerator6
      (return (Variables|Teams|GetGolf)))))