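; Base enemy character that loads its combat and movement stats from DT_Enemy and exposes range, patrol route and speed helpers.
; TakeDamage applies knockback, lowers health, grants player gauge points and spawns floating damage text, with optional camera shake and timed post-process blur and aberration.
; Hit stop freezes every actor through CustomTimeDilation until a timer restores it.
; Die notifies listeners and destroys the actor but is not triggered here; Attack is empty.
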(event Custom|Die
  (Default|CallOnDie)
  (Actor|DestroyActor))

(event EventBeginPlay
  (bind _returnvalue (Utilities|GetDataTableRow "/Game/Enemies/Parent/DT_Enemy.DT_Enemy" (.rowname (Variables|Default|GetData)))
    (:then
      (bind _output_get (Variables|Stats|SetMaxHealth (.Health (Utilities|Struct|BreakFEnemy _returnvalue))))
      (Variables|Stats|SetHealth _output_get)
      (Variables|Stats|Attack|SetDamage (.Damage (Utilities|Struct|BreakFEnemy _returnvalue)))
      (Variables|Stats|Attack|SetAttack%20Speed (.AttackSpeed (Utilities|Struct|BreakFEnemy _returnvalue)))
      (Variables|STats||Speeds|SetWalkSpeed (.WalkSpeed (Utilities|Struct|BreakFEnemy _returnvalue)))
      (Variables|Stats||Ranges|SetDefend%20Range (.DefendRange (Utilities|Struct|BreakFEnemy _returnvalue)))
      (Variables|Stats||Ranges|SetAttack%20Range (.AttackRange (Utilities|Struct|BreakFEnemy _returnvalue)))
      (Variables|STats||Speeds|SetSprintSpeed (.SprintSpeed (Utilities|Struct|BreakFEnemy _returnvalue)))
      (Variables|STats||Speeds|SetStrafeSpeed (.StrafeSpeed (Utilities|Struct|BreakFEnemy _returnvalue)))
      (Variables|Default|SetSC%20See%20Player (.SC_SeePlayer (Utilities|Struct|BreakFEnemy _returnvalue))))))

(event EventTakeDamage
  (params (Damage :type Float%20%28double-precision%29) (GaugeGain :type Float%20%28double-precision%29) (KB%20Strength :type Float%20%28double-precision%29) (KB%20Direction :type Vector :default "0, 0, 0") (FreezeFrameDurationDuration :type Float%20%28double-precision%29) (RadialBlurDuration :type Float%20%28double-precision%29) (ChromaAberrationDuration :type Float%20%28double-precision%29) (FreezeFrame :type Boolean) (CameraShake :type Boolean) (RadialBlur :type Boolean) (ChromaAberration :type Boolean))
  (bind _returnvalue (Transformation|GetActorLocation))
  (bind _mesh (Variables|Character|GetMesh))
  (bind _ui_offset (Variables|Default|GetUI%20Offset))
  (Components|Movement|StopMovementImmediately (Variables|Character|GetCharacterMovement))
  (CallFunction|TakeKnockback KB%20Strength KB%20Direction)
  ;[0.1406 0.01245 0.0154 0.85] Take Damage
  (Variables|Default|SetHurt true)
  (Development|PrintString (Utilities|String|ToString(Float) (Variables|Stats|GetHealth)))
  (Variables|Stats|SetHealth (- (Variables|Stats|GetHealth) Damage))
  (bind _asbp_player (Utilities|Casting|CastToBP_Player (Game|GetPlayerCharacter 0)))
  (Default|GainGaugePoints _asbp_player GaugeGain)
  ;[1 0.3061 0.7206] UI Damage text
  (bind _returnvalue_2 (Game|SpawnActorfromClass "/Game/UI/FX/BP_DamageText.BP_DamageText_C" (Math|Transform|MakeTransform (Math|Vector|MakeVector (Math|Random|RandomFloatinRange (- (.x _returnvalue) _ui_offset) (+ (.x _returnvalue) _ui_offset)) (Math|Random|RandomFloatinRange (- (.y _returnvalue) _ui_offset) (+ (.y _returnvalue) _ui_offset)) (.z _returnvalue)) "0, 0, 0" "1.000000,1.000000,1.000000") "Undefined" "MultiplyWithRoot" 0 0))
  (bind _aswbp_uidamage (Utilities|Casting|CastToWBP_UIDamage (UserInterface|GetWidget (Variables|/Game/UI/FX/BP_DamageText.BP_DamageText_C|GetWBP_DamageWidget _returnvalue_2))))
  (Variables|/Game/UI/FX/WBP_UIDamage.WBP_UIDamage_C|SetDamage _aswbp_uidamage (Utilities|Text|ToText(Float) Damage "HalfToEven"))
  (if RadialBlur
    (bind _outactors (Actor|GetAllActorsOfClasswithTag "/Script/Engine.PostProcessVolume" "RadialBlur"))
    (bind _output_get (Variables|PPV|SetPPV_RadialBlur (Utilities|Array|Get(acopy) _outactors)))
    (Variables|/Script/Engine.PostProcessVolume|SetbEnabled _output_get true)
    (Utilities|Time|SetTimerbyFunctionName 0 "EndRadialBlur" RadialBlurDuration))
  (if ChromaAberration
    (bind _outactors_2 (Actor|GetAllActorsOfClasswithTag "/Script/Engine.PostProcessVolume" "ChromaticAberration"))
    (bind _output_get_2 (Variables|PPV|SetPPV_ChromaticAberration (Utilities|Array|Get(acopy) _outactors_2)))
    (Variables|/Script/Engine.PostProcessVolume|SetbEnabled _output_get_2 true)
    (Utilities|Time|SetTimerbyFunctionName 0 "EndChromaticAberration" ChromaAberrationDuration))
  ;[0.07421 0.002732 0.002428] Game feel
  (if CameraShake
    (Camera|PlayWorldCameraShake "/Game/FX/Effects/Camera/CS_TakeDamage.CS_TakeDamage_C" (Transformation|GetActorLocation) 0.0 1e+05 0.0))
  (if FreezeFrame
    (CallFunction|StartHitStop FreezeFrameDurationDuration)
    (Rendering|Material|SetOverlayMaterial _mesh "/Game/Enemies/Parent/MI_Hurt.MI_Hurt" :!class /Script/Engine.MeshComponent)
    (Utilities|FlowControl|Delay 0.3)
    (Rendering|Material|SetOverlayMaterial _mesh 0 :!class /Script/Engine.MeshComponent)))

(event EventAttack)

(fn ConstructionScript)

(fn StartHitStop
  (params (FFTime :type Float%20%28single-precision%29))
  (if (<= FFTime 0.0)
    (bind _outactors (Actor|GetAllActorsOfClass "/Script/Engine.Actor"))
    (for _array_element _outactors
      (Variables|/Script/Engine.Actor|SetCustomTimeDilation _array_element 0.0)
      (Utilities|Time|SetTimerbyFunctionName 0 "EndHitStop" 0.01))
    (else
      (bind _outactors_2 (Actor|GetAllActorsOfClass "/Script/Engine.Actor"))
      (for _array_element_2 _outactors_2
        (Variables|/Script/Engine.Actor|SetCustomTimeDilation _array_element_2 0.0)
        (Utilities|Time|SetTimerbyFunctionName 0 "EndHitStop" FFTime)))))

(fn EndHitStop
  (bind _outactors (Actor|GetAllActorsOfClass "/Script/Engine.Actor"))
  (for _array_element _outactors
    (Variables|/Script/Engine.Actor|SetCustomTimeDilation _array_element 1.0)))

(fn TakeKnockback
  (params (KB%20Strength :type Float%20%28double-precision%29) (KB%20Direction :type Vector))
  (Character|LaunchCharacter (* KB%20Strength KB%20Direction) true true))

(fn EndRadialBlur
  (Variables|/Script/Engine.PostProcessVolume|SetbEnabled (Variables|PPV|GetPPV_RadialBlur) false))

(fn EndChromaticAberration
  (Variables|/Script/Engine.PostProcessVolume|SetbEnabled (Variables|PPV|GetPPV_ChromaticAberration) false))

(fn GetIdealRange
  (return (Variables|Stats||Ranges|GetAttack%20Range) (Variables|Stats||Ranges|GetDefend%20Range)))

(fn GetPatrolRoute
  (return (Variables|AI|GetPatrolRoute)))

(fn SetMovementSpeed
  (params (Speed :type E_MovementSpeed%20Enum :default "NewEnumerator0"))
  (bind _output_get (Variables|/Script/Engine.CharacterMovementComponent|SetMaxWalkSpeed (Variables|Character|GetCharacterMovement) (Utilities|Select :Index Speed :NewEnumerator0 (Variables|STats||Speeds|GetIdleSpeed) :NewEnumerator1 (Variables|STats||Speeds|GetWalkSpeed) :NewEnumerator2 (Variables|STats||Speeds|GetStrafeSpeed) :NewEnumerator3 (Variables|STats||Speeds|GetSprintSpeed))))
  (return _output_get))