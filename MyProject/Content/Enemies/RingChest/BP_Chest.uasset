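; Ring chest built on a damageable parent: it is broken by hits and offers a choice of two rings on death.
; Each accepted hit passes fixed damage to the parent; surviving hits play a timeline that wobbles and scales the mesh.
; Death opens WBP_PickupChoice, freezes global time, fills it with two independently random LootableRings looked up in DT_Item, then destroys the chest.
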(event EventBeginPlay
  (|CallParentFunction)
  (Components|Activation|Deactivate (Variables|Character|GetCharacterMovement)))

(event EventTakeDamage
  (params (Damage :type Float%20%28double-precision%29) (GaugeGain :type Float%20%28double-precision%29) (KB%20Strength :type Float%20%28double-precision%29) (KB%20Direction :type Vector :default "0, 0, 0") (FreezeFrameDurationDuration :type Float%20%28double-precision%29) (RadialBlurDuration :type Float%20%28double-precision%29) (ChromaAberrationDuration :type Float%20%28double-precision%29) (FreezeFrame :type Boolean) (CameraShake :type Boolean) (RadialBlur :type Boolean) (ChromaAberration :type Boolean))
  (bind _chest (Variables|Default|GetChest))
  (Transformation|SetMobility (Variables|Default|GetChest) "Movable")
  (if (Variables|Default|GetCanTakeDamage)
    (|CallParentFunction 1.0 0.0 0.0 "0, 0, 0" 0.001 0.1 0.1 false true true true)
    (if (<= (Variables|Default|GetHealth) 0.0)
      (CallFunction|Die)
      (else
        (bind (_direction _jump _vibre _grossis_r2tr2ci) (Timeline|Timeline PlayFromStart)
          (:Update
            (Transformation|SetRelativeRotation _chest (Math|Rotator|MakeRotator 0.0 (* _vibre 15.0) 0.0) false false)
            (Transformation|SetWorldScale3D _chest (Math|Conversions|ToVector(Float) (* _grossis_r2tr2ci 0.5))))
          (:Finished
            (Transformation|SetMobility (Variables|Default|GetChest) "Static")))))))

(event EventDie
  (Default|CallOnDie self)
  (bind _returnvalue (UserInterface|CreateWidget "/Game/UI/PickUp/WBP_PickupChoice.WBP_PickupChoice_C"))
  (UserInterface|Viewport|AddtoViewport _returnvalue 0)
  (Utilities|Time|SetGlobalTimeDilation 0.0)
  (Utilities|FlowControl|Sequence
    (:then_0
      (bind _output_get (Variables|Default|SetRandomRing (.OutItem (Utilities|Array|Random (Variables|Default|GetLootableRings)))))
      (bind _returnvalue_2 (Utilities|GetDataTableRow "/Game/Inventory/DT_Item.DT_Item" (.RowName (Utilities|Struct|BreakDataTableRowHandle _output_get)))
        (:then
          (Default|SetUIRing _returnvalue (.Artwork (Utilities|Struct|BreakF_Item _returnvalue_2)) (.RowName (Utilities|Struct|BreakDataTableRowHandle _output_get)) (.Description (Utilities|Struct|BreakF_Item _returnvalue_2)) 0 (.Ring (Utilities|Struct|BreakF_Item _returnvalue_2))))))
    (:then_1
      (bind _output_get_2 (Variables|Default|SetRandomRing (.OutItem (Utilities|Array|Random (Variables|Default|GetLootableRings)))))
      (bind _returnvalue_3 (Utilities|GetDataTableRow "/Game/Inventory/DT_Item.DT_Item" (.RowName (Utilities|Struct|BreakDataTableRowHandle _output_get_2)))
        (:then
          (Default|SetUIRing _returnvalue (.Artwork (Utilities|Struct|BreakF_Item _returnvalue_3)) (.RowName (Utilities|Struct|BreakDataTableRowHandle _output_get_2)) (.Description (Utilities|Struct|BreakF_Item _returnvalue_3)) 1 (.Ring (Utilities|Struct|BreakF_Item _returnvalue_3)))
          (CallFunction|EndHitStop)
          (Actor|DestroyActor))))))

(fn ConstructionScript
  (|CallParentFunction))