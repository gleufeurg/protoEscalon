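; BP_Enemy_Sandbag is an enemy character Blueprint that provides hit stop and exposes combat range, patrol and movement data.
; Hit stop freezes both itself and player 0 through CustomTimeDilation, then separate named timers restore each to normal speed.
; Getters return attack and defend ranges and the patrol route, while SetMovementSpeed maps a speed state to the character's max walk speed.
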(fn ConstructionScript)

(fn StartHitStop
  (params (EnemyTime :type Float%20%28single-precision%29) (PlayerTime :type Float%20%28double-precision%29))
  (Variables|/Script/Engine.Actor|SetCustomTimeDilation (Game|GetPlayerCharacter 0) 0.0)
  (Variables|Default|SetCustomTimeDilation 0.0)
  (Utilities|Time|SetTimerbyFunctionName 0 "EndSelfHitStop" EnemyTime)
  (Utilities|Time|SetTimerbyFunctionName 0 "EndPlayerHitStop" PlayerTime))

(fn EndSelfHitStop
  (Variables|Default|SetCustomTimeDilation 1.0))

(fn EndPlayerHitStop
  (Variables|/Script/Engine.Actor|SetCustomTimeDilation (Game|GetPlayerCharacter 0) 1.0))

(fn GetIdealRange
  (return (Variables|Stats||Ranges|GetAttack%20Range) (Variables|Stats||Ranges|GetDefend%20Range)))

(fn GetPatrolRoute
  (return (Variables|AI|GetPatrolRoute)))

(fn SetMovementSpeed
  (params (Speed :type E_MovementSpeed%20Enum :default "NewEnumerator0"))
  (bind _output_get (Variables|/Script/Engine.CharacterMovementComponent|SetMaxWalkSpeed (Variables|Character|GetCharacterMovement) (Utilities|Select :Index Speed :NewEnumerator0 (Variables|STats||Speeds|GetIdleSpeed) :NewEnumerator1 (Variables|STats||Speeds|GetWalkSpeed) :NewEnumerator2 (Variables|STats||Speeds|GetStrafeSpeed) :NewEnumerator3 (Variables|STats||Speeds|GetSprintSpeed))))
  (return _output_get))